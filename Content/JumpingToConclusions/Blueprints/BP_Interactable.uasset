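; BP_Interactable is an interactable actor that registers itself with a BP_ThirdPersonCharacter standing inside its box trigger.
; On begin overlap, if no player is held, it stores the character as InteractingPlayer, sets that character's InteractableRef to itself and flags PlayerOverlap.
; End overlap clears both references and the flag only for that same character, so one player holds it at a time.
; The file defines no interaction behavior itself.
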(event `self.Box.OnComponentBeginOverlap`
  (params (OverlappedComponent :type "PrimitiveComponent Object Reference") (OtherActor :type "Actor Object Reference") (OtherComp :type "PrimitiveComponent Object Reference") (OtherBodyIndex :type Integer) (bFromSweep :type Boolean) (SweepResult :type "HitResult Structure (by ref)"))
  (`/Engine/EditorBlueprintResources/StandardMacros.IsValid` (`self.InteractingPlayer`)
    (:`Is Not Valid`
      (bind _asbp_third_person_character (cast `/Game/JumpingToConclusions/Blueprints/BP_ThirdPersonCharacter` OtherActor))
      (set `self.InteractingPlayer` _asbp_third_person_character)
      (set `/Game/JumpingToConclusions/Blueprints/BP_ThirdPersonCharacter.InteractableRef` self _asbp_third_person_character)
      (set `self.bPlayerOverlap` true))))

(event `self.Box.OnComponentEndOverlap`
  (params (OverlappedComponent :type "PrimitiveComponent Object Reference") (OtherActor :type "Actor Object Reference") (OtherComp :type "PrimitiveComponent Object Reference") (OtherBodyIndex :type Integer))
  (bind _asbp_third_person_character (cast `/Game/JumpingToConclusions/Blueprints/BP_ThirdPersonCharacter` OtherActor))
  (if (== _asbp_third_person_character (`self.InteractingPlayer`))
    (set `self.InteractingPlayer` null)
    (set `/Game/JumpingToConclusions/Blueprints/BP_ThirdPersonCharacter.InteractableRef` null _asbp_third_person_character)
    (set `self.bPlayerOverlap` false)))

(fn `UserConstructionScript`)