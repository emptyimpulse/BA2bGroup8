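; BP_SimonSays is a Simon Says sound puzzle that generates a random sequence of four color-coded beeps.
; When the interacting player begins overlapping its Box, it clears the interaction references, then appends eleven random values, calling PlayRound after each.
; PlayRound plays beeps for the first three entries and, after a Delay, passes the sequence to the player character's GetPuzzleAnswers.
; The Delay follows each sound inside the loop, so beeps are not spaced apart.
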(event `self.Box.OnComponentBeginOverlap`
  (params (OverlappedComponent :type "PrimitiveComponent Object Reference") (OtherActor :type "Actor Object Reference") (OtherComp :type "PrimitiveComponent Object Reference") (OtherBodyIndex :type Integer) (bFromSweep :type Boolean) (SweepResult :type "HitResult Structure (by ref)"))
  (bind _asbp_third_person_character (cast `/Game/JumpingToConclusions/Blueprints/BP_ThirdPersonCharacter` OtherActor))
  (if (== _asbp_third_person_character (`self.InteractingPlayer`))
    (set `self.InteractingPlayer` null)
    (set `/Game/JumpingToConclusions/Blueprints/BP_ThirdPersonCharacter.InteractableRef` null _asbp_third_person_character)
    (set `self.bPlayerOverlap` false)
    (for _ (range 11)
      (`KismetArrayLibrary.Array_Add` (`self.Buttons Pressed`) (`KismetMathLibrary.RandomIntegerInRange` 0 3))
      (`self.PlayRound` 3))))

(event `PlayRound`
  (params (Rounds :type Integer))
  (for _index (range (+ (+ Rounds -1) 1))
    (switch `int` (`|GetArrayItem` (`self.Buttons Pressed`) _index)
      (:`0`
        (`GameplayStatics.PlaySound2D` "/Game/Audio/Red_Beep.Red_Beep" 1.0 1.0 0.0 null null))
      (:`1`
        (`GameplayStatics.PlaySound2D` "/Game/Audio/Green_Beep.Green_Beep" 1.0 1.0 0.0 null null))
      (:`2`
        (`GameplayStatics.PlaySound2D` "/Game/Audio/Blue_Beep.Blue_Beep" 1.0 1.0 0.0 null null))
      (:`3`
        (`GameplayStatics.PlaySound2D` "/Game/Audio/Yellow_Beep.Yellow_Beep" 1.0 1.0 0.0 null null)))
    (`KismetSystemLibrary.Delay` 1.0)
    (bind _asbp_third_person_character (cast `/Game/JumpingToConclusions/Blueprints/BP_ThirdPersonCharacter` (`GameplayStatics.GetPlayerCharacter` 0)))
    (`/Game/JumpingToConclusions/Blueprints/BP_ThirdPersonCharacter.GetPuzzleAnswers` _asbp_third_person_character (`self.Buttons Pressed`))))

(fn `UserConstructionScript`
  (`parent.UserConstructionScript`))