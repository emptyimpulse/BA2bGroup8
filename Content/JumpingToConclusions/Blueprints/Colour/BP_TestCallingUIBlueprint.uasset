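; A test colour-matching puzzle Blueprint that checks an RGB value against a stored observer colour.
; GetColour stores the observer colour, while UpdateColour has an empty body but supplies R, G and B inputs.
; The check event treats the RGB difference as a vector, passing within a distance threshold.
; It prints YES or NO, and a match adds solved-puzzle score through JTCGameState.
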(event `GetColour`
  (params (ObserverColour :type "LinearColor Structure"))
  (bind _output_get (set `self.Observer Colour` ObserverColour)))

(event `check`
  (bind (_observer_colour_r _observer_colour_g _observer_colour_b) (break `LinearColor` (`self.Observer Colour`)))
  (if (<= (`KismetMathLibrary.VSize` (`KismetMathLibrary.MakeVector` (- (stale `UpdateColour` r) _observer_colour_r) (- (stale `UpdateColour` g) _observer_colour_g) (- (stale `UpdateColour` b) _observer_colour_b))) 0.5)
    (`KismetSystemLibrary.PrintString` " YES")
    (bind _asjtcgame_state (cast `JTCGameState` (`GameplayStatics.GetGameState`)))
    (`JTCGameState.AddSolvedPuzzleScore` _asjtcgame_state true)
    (else
      (`KismetSystemLibrary.PrintString` "NO"))))

(event `UpdateColour`
  (params (r :type "Float (double-precision)") (g :type "Float (double-precision)") (b :type "Float (double-precision)")))

(fn `NewFunction`)

(fn `UserConstructionScript`)