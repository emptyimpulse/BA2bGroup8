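; BP_Box is a test actor that shows network authority and replication state as text.
; On BeginPlay it sets TextAuthority to show whether this instance has authority.
; Every Tick it writes the current value of ReplicatedVar into the RepVar text, so server and client values can be compared.
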(event `self.ReceiveTick`
  (params (DeltaSeconds :type "Float (single-precision)"))
  (`TextRenderComponent.K2_SetText` (`self.RepVar`) (`KismetTextLibrary.Conv_StringToText` (`KismetStringLibrary.Concat_StrStr` "ReplicatedVar: " (`KismetStringLibrary.Conv_DoubleToString` (`self.ReplicatedVar`))))))

(event `self.ReceiveBeginPlay`
  (if (`self.HasAuthority`)
    (`TextRenderComponent.K2_SetText` (`self.TextAuthority`) (`KismetTextLibrary.Conv_StringToText` "HasAuthority"))
    (else
      (`TextRenderComponent.K2_SetText` (`self.TextAuthority`) (`KismetTextLibrary.Conv_StringToText` "No Authority")))))

(fn `UserConstructionScript`)