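; BP_NotBorkenObserver is a test Blueprint that shows a widget while the local player's character is within interaction range.
; The widget starts hidden on BeginPlay, and InteractDistance overlap begin and end events show and hide it.
; Both events respond only to a JumpingToConclusionsCharacter whose controller is player controller 0.
; The file only toggles visibility and contains no interaction logic.
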(event `self.ReceiveBeginPlay`
  (`SceneComponent.SetVisibility` (`self.Widget`) false false))

(event `self.InteractDistance.OnComponentBeginOverlap`
  (params (OverlappedComponent :type "PrimitiveComponent Object Reference") (OtherActor :type "Actor Object Reference") (OtherComp :type "PrimitiveComponent Object Reference") (OtherBodyIndex :type Integer) (bFromSweep :type Boolean) (SweepResult :type "HitResult Structure (by ref)"))
  (bind _asjumping_to_conclusions_character (cast `JumpingToConclusionsCharacter` OtherActor))
  (if (== (`Pawn.GetController` _asjumping_to_conclusions_character) (`GameplayStatics.GetPlayerController` 0))
    (`SceneComponent.SetVisibility` (`self.Widget`) true false)))

(event `self.InteractDistance.OnComponentEndOverlap`
  (params (OverlappedComponent :type "PrimitiveComponent Object Reference") (OtherActor :type "Actor Object Reference") (OtherComp :type "PrimitiveComponent Object Reference") (OtherBodyIndex :type Integer))
  (bind _asjumping_to_conclusions_character (cast `JumpingToConclusionsCharacter` OtherActor))
  (if (== (`GameplayStatics.GetPlayerController` 0) (`Pawn.GetController` _asjumping_to_conclusions_character))
    (`SceneComponent.SetVisibility` (`self.Widget`) false false)))

(fn `UserConstructionScript`)