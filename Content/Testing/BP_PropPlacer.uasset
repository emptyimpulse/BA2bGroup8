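; BP_PropPlacer is a testing Blueprint that sets up a prop from an array of meshes when its Activate event fires.
; Activate loops through MeshArray and assigns the entry whose index matches Option to the StaticMesh component.
; It then calls three flag-gated functions that randomise relative location, rotation and scale.
; Location and scale use multiplied random unit vectors, so scale is non-uniform and can go negative.
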(event `Activate`
  (for (_array_element _array_index) (`self.MeshArray`)
    (if (== (`self.Option`) _array_index)
      (`StaticMeshComponent.SetStaticMesh` (`self.StaticMesh`) _array_element)
      (`self.RandomisePosition`)
      (`self.RandomiseRotaion`)
      (`self.RandomScale`))))

(fn `RandomisePosition`
  (if (`self.Random Position`)
    (`SceneComponent.K2_SetRelativeLocation` (`self.StaticMesh`) (* (`KismetMathLibrary.RandomUnitVector`) 100.0) false false)))

(fn `RandomiseRotaion`
  (if (`self.Random rotation`)
    (`SceneComponent.K2_SetRelativeRotation` (`self.StaticMesh`) (`KismetMathLibrary.RandomRotator` false) false false)))

(fn `RandomScale`
  (if (`self.Random Scale`)
    (`SceneComponent.SetRelativeScale3D` (`self.StaticMesh`) (* (`KismetMathLibrary.RandomUnitVector`) 5.0))))

(fn `UserConstructionScript`)